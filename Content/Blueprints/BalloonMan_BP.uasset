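; BalloonMan is a steerable character that moves forward continuously on its own.
; Tick pushes it along its local X axis by Speed, scaled by delta time, with a swept offset for collision.
; The TurnRight and TurnLeft axis events share one yaw rotation, driven by summed axis values, TurnSpeed and world delta seconds.
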(event `self.ReceiveTick`
  (params (DeltaSeconds :type "Float (single-precision)"))
  ;[1 1 1] Move
  (`self.K2_AddActorLocalOffset` (`KismetMathLibrary.MakeVector` (* DeltaSeconds (`self.speed`))) true))

(event `InputAxis|TurnRight`
  (params (AxisValue :type "Float (single-precision)"))
  ;[1 1 1] Turn
  (`self.K2_AddActorLocalRotation` (`KismetMathLibrary.MakeRotator` 0.0 0.0 (* (+ AxisValue (stale `InputAxis|TurnLeft` AxisValue)) (`self.turnSpeed`) (`GameplayStatics.GetWorldDeltaSeconds`))) :!label _label))

(event `InputAxis|TurnLeft`
  (params (AxisValue :type "Float (single-precision)"))
  ;[1 1 1] Turn
  (goto _label))

(fn `UserConstructionScript`)