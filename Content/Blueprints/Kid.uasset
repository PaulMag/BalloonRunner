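; Kid is a chasing enemy actor that homes in on the player pawn, shown as a billboarded plane.
; Each tick it moves forward at Speed and turns at TurnSpeed toward the player, using GetYawBetweenActors to get a wrapped signed yaw difference.
; Its Plane component yaws to face the camera.
; Overlapping an actor of the player pawn's class only prints "DEAD", with no actual kill logic.
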(event `self.ReceiveBeginPlay`
  ;[1 1 1] Store player pawn
  (set `self.playerPawn` (`GameplayStatics.GetPlayerPawn` 0)))

(event `self.ReceiveActorBeginOverlap`
  (params (OtherActor :type "Actor Object Reference"))
  ;[1 1 1] Kill player on overlap
  (if (`KismetMathLibrary.ClassIsChildOf` (`GameplayStatics.GetObjectClass` OtherActor) (`GameplayStatics.GetObjectClass` (`self.playerPawn`)))
    (`KismetSystemLibrary.PrintString` "DEAD")))

(event `self.ReceiveTick`
  (params (DeltaSeconds :type "Float (single-precision)"))
  (bind _turnspeed (`self.turnSpeed`))
  (`|ExecutionSequence`
    (:`then_0`
      ;[1 1 1] Move
      (`self.K2_AddActorLocalOffset` (`KismetMathLibrary.MakeVector` (* (`GameplayStatics.GetWorldDeltaSeconds`) (`self.speed`))))
      (if (> (`self.getYawBetweenActors` self (`self.playerPawn`)) 0.0)
        (set `self.currentTurnSpeed` (* _turnspeed 1.0))
        (else
          (set `self.currentTurnSpeed` (* _turnspeed -1.0))))
      (`self.K2_AddActorLocalRotation` (`KismetMathLibrary.MakeRotator` 0.0 0.0 (* (`self.currentTurnSpeed`) (`GameplayStatics.GetWorldDeltaSeconds`)))))
    (:`then_1`
      ;[1 1 1] Face plane towards camera
      (`SceneComponent.K2_SetWorldRotation` (`self.Plane`) (`KismetMathLibrary.MakeRotator` (.roll (`SceneComponent.K2_GetComponentRotation` (`self.Plane`))) (.pitch (`SceneComponent.K2_GetComponentRotation` (`self.Plane`))) (+ (.yaw (`KismetMathLibrary.FindLookAtRotation` (`self.K2_GetActorLocation`) (`PlayerCameraManager.GetCameraLocation` (`GameplayStatics.GetPlayerCameraManager` 0)))) -90.0)) false false))))

(fn `getYawBetweenActors`
  (params (vector1 :type "Actor Object Reference") (vector2 :type "Actor Object Reference"))
  (returns (angleDeg :type "Float (double-precision)"))
  (bind _returnvalue (- (.yaw (`KismetMathLibrary.FindLookAtRotation` (`self.K2_GetActorLocation` vector1) (`self.K2_GetActorLocation` vector2))) (.yaw (`self.K2_GetActorRotation`))))
  (if (> _returnvalue 180.0)
    (return (- _returnvalue 360.0))
    (elif (< _returnvalue -180.0)
      (return (+ _returnvalue 360.0))
      (else
        (return _returnvalue)))))

(fn `UserConstructionScript`)