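; Game mode Blueprint that keeps spawning Kid actors as enemies around the player.
; On BeginPlay a looping timer calls SpawnEnemy every spawn period.
; Each spawn picks a random X/Y offset within a square range around the first player pawn at its height, with random yaw.
; Spawns adjust for collisions where possible but always happen, and nothing here caps their number.
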(event `spawnEnemyEvent`
  (`self.spawnEnemy`))

(event `self.ReceiveBeginPlay`
  (`KismetSystemLibrary.K2_SetTimerDelegate` (delegate `spawnEnemyEvent`) (`self.emenySpawnPeriod`) true))

(fn `spawnEnemy`
  (bind _enemyspawnrange (`self.enemySpawnRange`))
  (bind _returnvalue (* -1.0 _enemyspawnrange))
  (`|SpawnActorFromClass` "/Game/Blueprints/Kid.Kid_C" (`KismetMathLibrary.MakeTransform` (+ (`self.K2_GetActorLocation` (`GameplayStatics.GetPlayerPawn` 0)) (`KismetMathLibrary.MakeVector` (`KismetMathLibrary.RandomFloatInRange` _returnvalue _enemyspawnrange) (`KismetMathLibrary.RandomFloatInRange` _returnvalue _enemyspawnrange))) (`KismetMathLibrary.MakeRotator` 0.0 0.0 (`KismetMathLibrary.RandomFloatInRange` 0.0 360.0))) "AdjustIfPossibleButAlwaysSpawn" "OverrideRootScale" null null))

(fn `UserConstructionScript`)